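; A HUD Blueprint that draws a UI through a custom Frames library rather than UMG, apparently as a test with placeholder names and text.
; On BeginPlay it creates a local configuration with a default font, builds a Frames environment, and adds a colored frame and child text, both center-pinned to the root.
; DrawHUD renders the stored environment each frame at the current screen size.
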(event EventDrawHUD
  (params (SizeX :type Integer) (SizeY :type Integer))
  (Class|FramesEnvironment|Render (Variables|Default|Getenv) SizeX SizeY))

(event EventBeginPlay
  (bind _returnvalue (Class|FramesLibrary|FramesConfigurationLocalCreate))
  (Class|FramesConfigurationLocal|Initialize _returnvalue)
  (Class|FramesConfigurationLocal|FontDefaultIdSet _returnvalue "/Game/Test/LindenHill.LindenHill")
  (bind _returnvalue_2 (Class|FramesLibrary|FramesEnvironmentCreate _returnvalue))
  (Variables|Default|Setenv _returnvalue_2)
  (bind _returnvalue_3 (Class|FramesLibrary|FramesFrameCreate (Class|FramesEnvironment|RootGet _returnvalue_2) "ttt"))
  (Class|FramesFrame|BackgroundSet _returnvalue_3 "(R=0.720000,G=0.480661,B=0.565073,A=1.000000)")
  (Class|FramesFrame|PinSetAnchorAnchor _returnvalue_3 "EFA_CENTER" (Class|FramesEnvironment|RootGet _returnvalue_2) "EFA_CENTER")
  (bind _returnvalue_4 (Class|FramesLibrary|FramesTextCreate _returnvalue_3))
  (Class|FramesText|TextSet _returnvalue_4 "tttt")
  (Class|FramesFrame|PinSetAnchorAnchor _returnvalue_4 "EFA_CENTER" (Class|FramesEnvironment|RootGet _returnvalue_2) "EFA_CENTER")
  (Class|FramesText|FontSizeSet _returnvalue_4 4e+01))

(fn ConstructionScript)